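; BP_Ennemy is an enemy that chases the player and reacts when hit.
; On BeginPlay it caches the player's follow camera and animation Blueprint.
; When PawnSensing spots a ThirdPersonCharacter, it prints a debug message and uses AIMoveTo to approach player 0.
; GetHit checks the Hittable flag on the player's AnimBP, then plays a random montage from an array and calls CamShake.
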(event OnSeePawn(PawnSensing)
  (params (Pawn :type Pawn%20Object%20Reference))
  ;[1 1 1] On See Pawn
  (bind _asthird_person_character (Utilities|Casting|CastToThirdPersonCharacter Pawn))
  (Development|PrintString (Utilities|String|Append "I See" (Utilities|GetDisplayName _asthird_person_character)))
  (AI|AIMoveTo self "0, 0, 0" (Game|GetPlayerCharacter 0) 2.0 false))

(event Custom|GetHit
  (bind _montagearray (Variables|Default|GetMontageArray))
  ;[1 1 1] Get Hit
  (if (Variables|/Game/CloseCombatAnimSet/Mannequin/Animations/ThirdPerson_AnimBPBig.ThirdPerson_AnimBPBig_C|GetHittable? (Variables|Default|GetRefAnimBP))
    (Animation|PlayAnimMontage (Utilities|Array|Get(acopy) _montagearray (Math|Random|RandomInteger (Utilities|Array|Length _montagearray))) 1.0 "None")
    (CallFunction|CamShake)))

(event EventBeginPlay
  (bind _returnvalue (Game|GetPlayerCharacter 0))
  ;[1 1 1] Ref
  (bind _asthird_person_character (Utilities|Casting|CastToThirdPersonCharacter _returnvalue))
  (Variables|Default|SetREF_Cam (Variables|/Game/ThirdPersonBP/Blueprints/ThirdPersonCharacter.ThirdPersonCharacter_C|GetFollowCamera _asthird_person_character))
  (bind _asthird_person_anim_bpbig (Utilities|Casting|CastToThirdPerson_AnimBPBig (Components|SkeletalMesh|GetAnimInstance (Variables|/Script/Engine.Character|GetMesh _returnvalue))))
  (Variables|Default|SetRefAnimBP _asthird_person_anim_bpbig))

(fn ConstructionScript)